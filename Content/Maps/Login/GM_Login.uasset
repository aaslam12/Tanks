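; GM_Login is the game mode for the login map, which shows the login screen widget to the local player.
; PostLogin creates the widget for a local controller, adds it to the viewport, releases viewport mouse capture, focuses it and prints the result.
; BeginPlay caches the BP_TankGameInstance and prints its current game mode for debugging.
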(event EventBeginPlay
  (bind _asbp_tank_game_instance (Utilities|Casting|CastToBP_TankGameInstance (Game|GetGameInstance)))
  (bind _output_get (Variables|Default|SetGameInstance _asbp_tank_game_instance))
  (Utilities|IsValid _output_get
    (:Is%20Valid
      (Development|PrintString (Utilities|String|EnumtoString (Variables|/Script/Tanks.TankGameInstance|GetCurrentGameMode _output_get))))))

(event EventPostLogin
  (params (NewPlayer :type Player%20Controller%20Object%20Reference))
  (if (Pawn|IsLocalController NewPlayer)
    (bind _returnvalue (UserInterface|CreateWidget (Variables|Default|GetLoginScreenWidgetClass) NewPlayer))
    (bind _output_get (Variables|Default|SetLoginScreenWidget _returnvalue))
    (Utilities|IsValid _output_get
      (:Is%20Valid
        (UserInterface|Viewport|AddtoViewport _output_get 0)
        (Class|GameplayStatics|SetViewportMouseCaptureMode "NoCapture")
        (Widget|SetFocus _output_get)
        (Development|PrintString "Widget Added to Viewport"))
      (:Is%20Not%20Valid
        (Development|PrintString "Widget failed to add to Viewport")))))

(fn ConstructionScript)