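; GM_Tanks is the game mode for the tank game, handling mouse capture and player login setup.
; On BeginPlay it sets the viewport to capture the mouse permanently.
; On PostLogin it calls the parent handler, sets game-only input on the new controller, then prints the custom name and team from BP_TankPlayerState as debug text.
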(event EventBeginPlay
  (Class|GameplayStatics|SetViewportMouseCaptureMode "CapturePermanently"))

(event EventPostLogin
  (params (NewPlayer :type Player%20Controller%20Object%20Reference))
  (|CallParentFunction NewPlayer)
  (Input|SetInputModeGameOnly NewPlayer true)
  (bind _asbp_tank_player_state (Utilities|Casting|CastToBP_TankPlayerState (Variables|/Script/Engine.Controller|GetPlayerState NewPlayer)))
  (Development|PrintString (Utilities|String|Append "Player Name: " (Variables|/Script/Tanks.TankPlayerState|GetCustomPlayerName _asbp_tank_player_state) "Team: " (Utilities|String|EnumtoString (Variables|/Script/Tanks.TankPlayerState|GetCurrentTeam _asbp_tank_player_state))) true true "(R=0.000000,G=0.660000,B=1.000000,A=1.000000)" 1e+01))

(fn ConstructionScript)