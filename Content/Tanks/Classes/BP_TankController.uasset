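; Player controller for tanks that hosts a debug overlay and handles gun sight HUD input.
; It creates WB_Debug on BeginPlay and forwards debug circle draw requests to it.
; Mouse wheel up hides and down shows the GunSight in the TankPlayer's GunSightWidget.
; A hardcoded 5 key nudges the controlled tank's GunCenter slightly along X through its canvas slot and prints the offset position, apparently for calibration.
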(event Input|EnhancedActionEvents|EnhancedInputActionIA_MouseWheelUp
  (params (ActionValue :type Boolean) (ElapsedSeconds :type Float%20%28double-precision%29) (TriggeredSeconds :type Float%20%28double-precision%29) (InputAction :type Input%20Action%20Object%20Reference :default "/Game/Tanks/Input/IA/IA_MouseWheelUp.IA_MouseWheelUp"))
  (bind _gunsightwidget (Variables|/Game/Tanks/Classes/BP_Tank.BP_Tank_C|GetGunSightWidget (.AsBP%20Tank (Utilities|Casting|CastToBP_Tank (Variables|Default|GetTankPlayer))))
    (:then
      (bind _gunsight (Variables|/Game/Tanks/UI/GunSight/WB_GunSight.WB_GunSight_C|GetGunSight _gunsightwidget)
        (:then
          (Widget|SetVisibility _gunsight "Hidden"))
        (:else)))
    (:else)))

(event Input|EnhancedActionEvents|EnhancedInputActionIA_MouseWheelDown
  (params (ActionValue :type Boolean) (ElapsedSeconds :type Float%20%28double-precision%29) (TriggeredSeconds :type Float%20%28double-precision%29) (InputAction :type Input%20Action%20Object%20Reference :default "/Game/Tanks/Input/IA/IA_MouseWheelDown.IA_MouseWheelDown"))
  (bind _gunsightwidget (Variables|/Game/Tanks/Classes/BP_Tank.BP_Tank_C|GetGunSightWidget (.AsBP%20Tank (Utilities|Casting|CastToBP_Tank (Variables|Default|GetTankPlayer))))
    (:then
      (bind _gunsight (Variables|/Game/Tanks/UI/GunSight/WB_GunSight.WB_GunSight_C|GetGunSight _gunsightwidget)
        (:then
          (Widget|SetVisibility _gunsight "Visible"))
        (:else)))
    (:else)))

(event EventDrawDebugCircle
  (params (Position :type Vector%202D%20Structure%20%28by%20ref%29))
  (Default|DrawDebugCircle (Variables|Default|GetDebugWidget) Position))

(event EventBeginPlay
  (bind _returnvalue (UserInterface|CreateWidget "/Game/Tanks/UI/Debug/WB_Debug.WB_Debug_C" self))
  (Utilities|IsValid _returnvalue
    (:Is%20Valid
      (bind _output_get (Variables|Default|SetDebugWidget _returnvalue))
      (Utilities|IsValid _output_get
        (:Is%20Valid
          (UserInterface|Viewport|AddtoViewport _output_get 0))))))

(event Input|KeyboardEvents|5
  (params (Key :type Key%20Structure :default "None"))
  (bind _returnvalue (Pawn|GetControlledPawn))
  (bind _asbp_tank (Utilities|Casting|CastToBP_Tank _returnvalue))
  (bind _gunsightwidget (Variables|/Game/Tanks/Classes/BP_Tank.BP_Tank_C|GetGunSightWidget _asbp_tank))
  (bind _guncenter (Variables|/Game/Tanks/UI/GunSight/WB_GunSight.WB_GunSight_C|GetGunCenter _gunsightwidget))
  (bind _returnvalue_2 (Class|WidgetLayoutLibrary|SlotasCanvasSlot _guncenter))
  (bind _returnvalue_3 (Class|CanvasPanelSlot|GetPosition _returnvalue_2))
  (bind _returnvalue_4 (+ (.x _returnvalue_3) 0.5))
  (:Pressed
    (Class|CanvasPanelSlot|SetPosition _returnvalue_2 (Math|Vector2D|MakeVector2D _returnvalue_4 (.y _returnvalue_3)))
    (Development|PrintString (Utilities|String|ToString(Float) _returnvalue_4) true true "(R=0.000000,G=0.660000,B=1.000000,A=1.000000)" 5e+03)))

(fn ConstructionScript)